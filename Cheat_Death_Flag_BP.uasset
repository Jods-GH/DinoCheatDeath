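; ARK Cheat Death flag structure that lets players with structure access recall their team's listed dinos to it.
; On the server it registers in a per-team CustomActorList, updating that on team change or destruction.
; Its radial-menu entry spawns a helper actor with dino names and GPS coordinates from another tagged team list.
; DinoWasSelected matches that string by index, teleports the dino nearby and notifies the first team player found.
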(event EventBeginPlay
  (Utilities|FlowControl|Delay 0.2)
  (Variables|/Script/ShooterGame.PrimalInventoryComponent|SetbAllowRemoteInventory (Variables|Default|GetMyInventoryComponent) false)
  (Variables|Default|SetOld%20Team (Variables|Default|GetTargetingTeam) false)
  (Variables|Default|SetSelfRef self false)
  (if (not (Variables|Default|GetbIsPreviewStructure))
    (Utilities|SwitchNetAuthority
      (:DedicatedServer
        _)
      (:PlayerServer
        _))
    (CallFunction|RegisterCALCheatDeathFlag)
    (CallFunction|GetData)))

(event EventDestroyed
  (Utilities|SwitchNetAuthority
    (:DedicatedServer
      _)
    (:PlayerServer
      _))
  (CallFunction|DebugPrint "event destroyed")
  (Utilities|FlowControl|Sequence
    (:then_0
      (bind _returnvalue (Class|VictoryCore|GetCustomActorList (Class|Actor|GetWorld) (Utilities|String|StringToName (Utilities|String|Append (Variables|Default|GetCheatDeath%20TP) (Utilities|String|ToString(Integer) (Variables|Default|GetTargetingTeam))))))
      (Variables|Default|SetEnd_Cal _returnvalue)
      (CallFunction|DebugPrint "Event_destroyed get custom actor list"))
    (:then_1
      (Utilities|Array|RemoveItem (Variables|/Script/ShooterGame.CustomActorList|GetActorList (Variables|Default|GetEnd_Cal)) (Variables|Default|GetSelfRef))
      (if (Variables|Default|GetActivate%20Debug%20Print)
        (CallFunction|DebugPrint "Event_Destroyed item removed")
        (for _array_element (Variables|/Script/ShooterGame.CustomActorList|GetActorList (Variables|Default|GetEnd_Cal))
          (bind _asprimalstructureitemcontainer (Utilities|Casting|CastToPrimalStructureItemContainer _array_element))
          (CallFunction|DebugPrint (Utilities|String|Append "Event_Destroyed " (Variables|/Script/ShooterGame.PrimalStructureItemContainer|GetBoxName _asprimalstructureitemcontainer))))))))

(event EventDinoWasSelected
  (params (DinoToGoBackTo :type String))
  (bind _returnvalue (Transformation|GetActorLocation))
  (bind _selfref (Variables|Default|GetSelfRef))
  (bind (_x _y _z) (Math|Vector|BreakVector _returnvalue))
  (bind _boxname (Variables|/Script/ShooterGame.PrimalStructureItemContainer|GetBoxName _selfref))
  (bind _returnvalue_2 (Utilities|Text|ToText(String) _boxname))
  (bind _returnvalue_3 (Utilities|Text|TextIsEmpty _returnvalue_2))
  (bind _returnvalue_4 (Utilities|String|SelectString "CheatDeathFlag" _boxname _returnvalue_3))
  (CallFunction|DebugPrint (Utilities|String|Append "Event DinoWasSelected " DinoToGoBackTo))
  (bind (_array_element _array_index) (Utilities|Array|ForEachLoopwithBreak (Variables|Default|GetDinoListArray) :!label _label)
    (:LoopBody
      (if (Utilities|Enum|Equal(Enum) DinoToGoBackTo _array_element)
        (bind _dinolist (CallFunction|GetDinoList))
        (Utilities|IsValid (Utilities|Array|Get(acopy) (Variables|/Script/ShooterGame.CustomActorList|GetActorList _dinolist) _array_index)
          (:Is%20Valid
            (if (== _returnvalue "0, 0, 0")
              (CallFunction|DebugPrint (Utilities|String|Append "EventDinoWasSelected Actor Location not valid: " (Utilities|String|ToString(Vector) _returnvalue)))
              (else
                (Transformation|Teleport (Utilities|Array|Get(acopy) (Variables|/Script/ShooterGame.CustomActorList|GetActorList _dinolist) _array_index) (Math|Vector|MakeVector (+ _x 2.5e+02) (+ _y 2.5e+02) (+ _z 2.5e+02)) "0, 0, 0" true)
                (bind _asshootergamestate (Utilities|Casting|CastToShooterGameState (Game|GetGameState (Class|Actor|GetWorld)))
                  (:then
                    (bind _asprimaldinocharacter (Utilities|Casting|CastToPrimalDinoCharacter (Utilities|Array|Get(acopy) (Variables|/Script/ShooterGame.CustomActorList|GetActorList _dinolist) _array_index))
                      (:then
                        (bind _returnvalue_5 (Class|ShooterGameState|BaseGetAllShooterCharactersOfTeam _asshootergamestate (Variables|Default|GetTargetingTeam)))
                        (if (Utilities|Text|TextIsEmpty (Utilities|Text|ToText(String) (Variables|/Script/ShooterGame.PrimalDinoCharacter|GetTamedName _asprimaldinocharacter)))
                          (for _array_element_2 _returnvalue_5
                            (Class|ShooterPlayerController|ClientServerNotification (Variables|/Script/ShooterGame.ShooterCharacter|GetLastValidPlayerController _array_element_2) (Utilities|String|Append (Utilities|String|Append (Utilities|String|Append "Recalling " (Variables|/Script/ShooterGame.PrimalCharacter|GetDescriptiveName _asprimaldinocharacter)) " to ") _returnvalue_4) "(R=0.000000,G=0.014534,B=1.000000,A=1.000000)" 2.0 3.0)
                            (goto _label Break))
                          (else
                            (for _array_element_3 _returnvalue_5
                              (Class|ShooterPlayerController|ClientServerNotification (Variables|/Script/ShooterGame.ShooterCharacter|GetLastValidPlayerController _array_element_3) (Utilities|String|Append (Utilities|String|Append (Utilities|String|Append "Recalling " (Variables|/Script/ShooterGame.PrimalDinoCharacter|GetTamedName _asprimaldinocharacter)) " to ") _returnvalue_4) "(R=0.000000,G=0.014534,B=1.000000,A=1.000000)" 2.0 3.0)
                              (goto _label Break)))))
                      (:CastFailed
                        (CallFunction|DebugPrint "Event_FlagWasSelected cast to PrimalDinoCharacter failed"))))
                  (:CastFailed
                    (CallFunction|DebugPrint "Event_DinoWasSelected cast to shooter game state failed"))))))
          (:Is%20Not%20Valid
            (CallFunction|DebugPrint "Event_DinoWasSelected dino not valid")
            (CallFunction|DebugPrint (Utilities|String|BuildString(Integer) (Utilities|String|BuildString(Integer) "Evvent_DinoWasSelected " "ArrayItemToGet" _array_index) "ArrayLength: " (Utilities|Array|Length (Variables|/Script/ShooterGame.CustomActorList|GetActorList _dinolist))))))))))

(fn ConstructionScript
  (|CallParentFunction))

(fn RegisterCALCheatDeathFlag
  (bind _targetingteam (Variables|Default|GetTargetingTeam))
  (bind _cheatdeath_tp (Variables|Default|GetCheatDeath%20TP))
  (bind _returnvalue (Utilities|String|ToString(Integer) _targetingteam))
  (bind _returnvalue_2 (Utilities|String|Append _cheatdeath_tp _returnvalue))
  (bind _returnvalue_3 (Utilities|String|StringToName _returnvalue_2))
  (Utilities|FlowControl|Sequence
    (:then_0
      (bind _returnvalue_4 (Class|VictoryCore|GetCustomActorList (Class|Actor|GetWorld) _returnvalue_3))
      (Variables|Default|SetL_CAL _returnvalue_4 false))
    (:then_1
      (Utilities|IsValid (Variables|Default|GetL_CAL)
        (:Is%20Not%20Valid
          (bind _returnvalue_5 (Game|SpawnActorfromClass "/Script/ShooterGame.CustomActorList" (Transformation|GetActorTransform) false 0))
          (Variables|/Script/Engine.Actor|SetCustomTag _returnvalue_5 _returnvalue_3)
          (Variables|Default|SetL_CAL _returnvalue_5 false))))
    (:then_2
      (Utilities|Array|Add (Variables|/Script/ShooterGame.CustomActorList|GetActorList (Variables|Default|GetL_CAL)) (Variables|Default|GetSelfRef))
      (if (Variables|Default|GetActivate%20Debug%20Print)
        (CallFunction|DebugPrint (Utilities|String|Append "RegisterCAL tag: " (Utilities|String|ToString(Name) _returnvalue_3)))
        (for _array_element (Variables|/Script/ShooterGame.CustomActorList|GetActorList (Variables|Default|GetL_CAL))
          (bind _asprimalstructureitemcontainer (Utilities|Casting|CastToPrimalStructureItemContainer _array_element)
            (:then
              (CallFunction|DebugPrint (Utilities|String|Append "RegisterCAL: " (Variables|/Script/ShooterGame.PrimalStructureItemContainer|GetBoxName _asprimalstructureitemcontainer))))
            (:CastFailed
              (CallFunction|DebugPrint "RegisterCal cast to PrimalStructureItemContainer failed"))))))))

(fn DebugPrint
  (params (thing_to_print :type String))
  (bind _returnvalue (Utilities|String|Append "DinoCheatDeath_flag " thing_to_print))
  (if (Class|VictoryCore|IsShipping)
    (bind _asshootergamemode (Utilities|Casting|CastToShooterGameMode (Game|GetGameMode))
      (:then
        (if (Variables|Default|GetActivate%20Debug%20Print)
          (Class|ShooterGameMode|PrinttoServerGameLog _asshootergamemode _returnvalue false)))
      (:CastFailed
        (Development|PrintString "Cheat_Death_flag DebugPrint Cast to Shooter GameMode failed")))
    (else
      (Development|PrintString _returnvalue))))

(fn BPTryMultiUse
  (params (ForPC :type Player%20Controller%20Object%20Reference) (UseIndex :type Integer))
  (switch int UseIndex
    (:Default
      _)
    (:298221
      (CallFunction|StartUI ForPC)))
  (return true))

(fn BPGetMultiUseEntries
  (params (ForPC :type Player%20Controller%20Object%20Reference) (MultiUseEntries :type Array%20of%20Multi%20Use%20Entry%20Structures))
  (bind _asprimalstructure (Utilities|Casting|CastToPrimalStructure (Variables|Default|GetSelfRef))
    (:then
      (bind _returnvalue (Class|PrimalStructure|AllowStructureAccess _asprimalstructure ForPC))
      (if _returnvalue
        (LocalVariables|SetMuBuffer MultiUseEntries)
        (Utilities|Array|Add (LocalVariables|GetMuBuffer) (Utilities|Struct|MakeMultiUseEntry 0 "Recall Dino to Flag " 298221 0 false false false false false false false false false true false false false false 0 "(B=175,G=175,R=175,A=255)" (Math|Color|MakeColor 135 200 255 255)))
        (else
          (CallFunction|DebugPrint "BPGetMultiUseEntry no Structure access")))
      (return (LocalVariables|GetMuBuffer)))
    (:CastFailed
      (CallFunction|DebugPrint "BPGetMultiUseEntry cast to PrimalStructure failed"))))

(fn StartUI
  (params (for%20PC :type Player%20Controller%20Object%20Reference))
  (bind _returnvalue (Pawn|GetControlledPawn for%20PC))
  (bind _dinolistarray (Variables|Default|GetDinoListArray))
  (bind _dinolistarray_2 (Variables|Default|GetDinoListArray))
  (CallFunction|DebugPrint "StartUI")
  (Utilities|IsValid _returnvalue
    (:Is%20Valid
      (bind _dinolist (CallFunction|GetDinoList))
      (if (== (Utilities|Array|Length (Variables|Default|GetDinoListArray)) (Utilities|Array|Length (Variables|/Script/ShooterGame.CustomActorList|GetActorList _dinolist)))
        _
        (else
          (Utilities|Array|Clear (Variables|Default|GetDinoListArray))
          (for _array_element (Variables|/Script/ShooterGame.CustomActorList|GetActorList _dinolist)
            (bind _asprimaldinocharacter (Utilities|Casting|CastToPrimalDinoCharacter _array_element)
              (:then
                (bind _returnvalue_2 (Class|VictoryCore|GetGPSCoords (Class|Actor|GetWorld) (Transformation|GetActorLocation _array_element)))
                (if (Utilities|Text|TextIsEmpty (Utilities|Text|ToText(String) (Variables|/Script/ShooterGame.PrimalDinoCharacter|GetTamedName _asprimaldinocharacter)))
                  (Utilities|Array|Add _dinolistarray_2 (Utilities|String|Append (Variables|/Script/ShooterGame.PrimalCharacter|GetDescriptiveName _asprimaldinocharacter) (Utilities|String|Append (Utilities|String|Append (Utilities|String|Append " Lat:" (Utilities|String|ToString(Text) (Utilities|Text|ToText(Float) (/ (.x _returnvalue_2) 1e+01) "HalfToEven"))) " | ") (Utilities|String|Append "Lon: " (Utilities|String|ToString(Text) (Utilities|Text|ToText(Float) (/ (.y _returnvalue_2) 1e+01) "HalfToEven"))))))
                  (else
                    (Utilities|Array|Add _dinolistarray_2 (Utilities|String|Append (Variables|/Script/ShooterGame.PrimalDinoCharacter|GetTamedName _asprimaldinocharacter) (Utilities|String|Append (Utilities|String|Append (Utilities|String|Append " Lat:" (Utilities|String|ToString(Text) (Utilities|Text|ToText(Float) (/ (.x _returnvalue_2) 1e+01) "HalfToEven"))) " | ") (Utilities|String|Append "Lon: " (Utilities|String|ToString(Text) (Utilities|Text|ToText(Float) (/ (.y _returnvalue_2) 1e+01) "HalfToEven")))))))))
              (:CastFailed
                (CallFunction|DebugPrint "StartUI cast to PrimalDinoCharacter failed"))))))
      (if (Variables|Default|GetActivate%20Debug%20Print)
        (for _array_element_2 _dinolistarray
          (CallFunction|DebugPrint (Utilities|String|Append "StartUI Dinolist: " _array_element_2))))
      (bind _returnvalue_3 (Game|SpawnActorfromClass "/Game/Mods/DinoCheatDeath/CheatDeath_RallyToFlag_com_Actor.CheatDeath_RallyToFlag_com_Actor_C" (Transformation|GetActorTransform _returnvalue) false for%20PC _dinolistarray self _returnvalue))
      (Actor|SetOwner _returnvalue_3 _returnvalue)
      (Default|Init _returnvalue_3))
    (:Is%20Not%20Valid
      (CallFunction|DebugPrint "StartUI object not valid"))))

(fn GetDinoList
  (bind _selfref (Variables|Default|GetSelfRef))
  (bind _targetingteam (Variables|/Script/Engine.Actor|GetTargetingTeam _selfref))
  (bind _returnvalue (Utilities|String|ToString(Integer) _targetingteam))
  (bind _returnvalue_2 (Utilities|String|Append "CheatDeathDinoList" _returnvalue))
  (bind _returnvalue_3 (Class|VictoryCore|GetCustomActorList (Class|Actor|GetWorld) (Utilities|String|StringToName _returnvalue_2)))
  (if (Variables|Default|GetActivate%20Debug%20Print)
    (CallFunction|DebugPrint (Utilities|String|Append "GetDinoList " _returnvalue_2))
    (for _array_element (Variables|/Script/ShooterGame.CustomActorList|GetActorList _returnvalue_3)
      (bind _asprimaldinocharacter (Utilities|Casting|CastToPrimalDinoCharacter _array_element)
        (:then
          (CallFunction|DebugPrint (Utilities|String|Append "GetDinoList item: " (Variables|/Script/ShooterGame.PrimalCharacter|GetDescriptiveName _asprimaldinocharacter))))
        (:CastFailed
          (Development|PrintString "GetDinoList cast to PrimalDinoCharacter failed")))))
  (return _returnvalue_3))

(fn BPChangedActorTeam
  (Utilities|SwitchNetAuthority
    (:DedicatedServer
      _)
    (:PlayerServer
      _))
  (CallFunction|DebugPrint "TargetTeamChanged")
  (Utilities|FlowControl|Sequence
    (:then_0
      (Utilities|IsValid (Variables|Default|GetTeam%20Changed%20Cal%20old)
        (:Is%20Not%20Valid
          (bind _returnvalue (Class|VictoryCore|GetCustomActorList (Class|Actor|GetWorld) (Utilities|String|StringToName (Utilities|String|Append (Variables|Default|GetCheatDeath%20TP) (Utilities|String|ToString(Integer) (Variables|Default|GetOld%20Team))))))
          (Variables|Default|SetTeam%20Changed%20Cal%20old _returnvalue false)
          (CallFunction|DebugPrint "BpChangedActor get Actor list"))))
    (:then_1
      (Utilities|Array|RemoveItem (Variables|/Script/ShooterGame.CustomActorList|GetActorList (Variables|Default|GetTeam%20Changed%20Cal%20old)) (Variables|Default|GetSelfRef))
      (if (Variables|Default|GetActivate%20Debug%20Print)
        (CallFunction|DebugPrint "BPChangedActor item  removed")
        (for _array_element (Variables|/Script/ShooterGame.CustomActorList|GetActorList (Variables|Default|GetTeam%20Changed%20Cal%20old))
          (bind _asprimalstructureitemcontainer (Utilities|Casting|CastToPrimalStructureItemContainer _array_element)
            (:then
              (CallFunction|DebugPrint (Utilities|String|Append "BpChangedActor List " (Variables|/Script/ShooterGame.PrimalStructureItemContainer|GetBoxName _asprimalstructureitemcontainer)))
              (Utilities|Array|Clear (Variables|/Script/ShooterGame.CustomActorList|GetActorList (Variables|Default|GetL_CAL)))
              (CallFunction|RegisterCALCheatDeathFlag)
              (Variables|Default|SetOld%20Team (Variables|Default|GetTargetingTeam) false))
            (:CastFailed
              (CallFunction|DebugPrint "BpChangedActor cast to PrimalStructureItemContainer failed"))))
        (else
          (Utilities|Array|Clear (Variables|/Script/ShooterGame.CustomActorList|GetActorList (Variables|Default|GetL_CAL)))
          (CallFunction|RegisterCALCheatDeathFlag)
          (Variables|Default|SetOld%20Team (Variables|Default|GetTargetingTeam) false))))))

(fn GetData
  (Utilities|SwitchNetAuthority
    (:DedicatedServer
      _)
    (:PlayerServer
      _))
  (if (Class|VictoryCore|IsShipping)
    (bind _asshootergamemode (Utilities|Casting|CastToShooterGameMode (Game|GetGameMode))
      (:then
        (Utilities|FlowControl|Sequence
          (:then_0
            (Class|ShooterGameMode|InitOptionBool _asshootergamemode "" "DinoCheatDeath" "ActivateDebugPrints" false))
          (:then_1
            (bind _returnvalue (Class|ShooterGameMode|GetBoolOptionIni _asshootergamemode "DinoCheatDeath" "ActivateDebugPrints" false))
            (Variables|Default|SetActivate%20Debug%20Print _returnvalue false)
            (CallFunction|DebugPrint "GetData finished"))))
      (:CastFailed
        (CallFunction|DebugPrint "GetData Cast to ShooterGameMode failed")))
    (else
      (Variables|Default|SetActivate%20Debug%20Print true false)
      (CallFunction|DebugPrint "GetData finished"))))